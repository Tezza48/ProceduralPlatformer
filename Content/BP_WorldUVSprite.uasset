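; BP_WorldUVSprite is a plane actor that drives its material's UV parameters from its transform, apparently to keep texture mapping consistent in world space.
; The construction script creates a dynamic material instance on the plane, then runs UpdateMaterial, which also runs on BeginPlay.
; UpdateMaterial sets U and V from X and Z scale and U Offset from world X in metres, while V Offset stays zero.
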(event `self.ReceiveBeginPlay`
  (`self.UpdateMaterial`))

(fn `UpdateMaterial`
  (bind _material (`self.Material`))
  (`MaterialInstanceDynamic.SetScalarParameterValue` _material "U" (.x (`self.GetActorScale3D`)))
  (`MaterialInstanceDynamic.SetScalarParameterValue` _material "V" (.z (`self.GetActorScale3D`)))
  (`MaterialInstanceDynamic.SetScalarParameterValue` _material "U Offset" (.x (/ (`self.K2_GetActorLocation`) 100.0)))
  (`MaterialInstanceDynamic.SetScalarParameterValue` _material "V Offset" 0.0))

(fn `UserConstructionScript`
  (bind _plane (`self.Plane`))
  (bind _returnvalue (`PrimitiveComponent.CreateDynamicMaterialInstance` _plane 0 (`PrimitiveComponent.GetMaterial` _plane 0)))
  (set `self.Material` _returnvalue)
  (`self.UpdateMaterial`))